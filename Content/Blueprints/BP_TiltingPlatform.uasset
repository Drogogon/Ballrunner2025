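; Platform actor that tilts while the player's Blueprintball pawn is inside its trigger box.
; Box begin overlap sets a tilting flag only for that pawn, while any end overlap clears it.
; Each Tick uses FInterpTo with scaled-down delta time to ease the Cube's relative roll toward TiltAngle, or back to level when the flag is off, holding pitch and yaw at zero.
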(event `self.Box.OnComponentBeginOverlap`
  (params (OverlappedComponent :type "PrimitiveComponent Object Reference") (OtherActor :type "Actor Object Reference") (OtherComp :type "PrimitiveComponent Object Reference") (OtherBodyIndex :type Integer) (bFromSweep :type Boolean) (SweepResult :type "HitResult Structure (by ref)"))
  (bind _asblueprintball (cast `/Game/Blueprints/Blueprintball` (`GameplayStatics.GetPlayerPawn` 0)))
  (if (== _asblueprintball OtherActor)
    (set `self.IsTilting` true)))

(event `self.Box.OnComponentEndOverlap`
  (params (OverlappedComponent :type "PrimitiveComponent Object Reference") (OtherActor :type "Actor Object Reference") (OtherComp :type "PrimitiveComponent Object Reference") (OtherBodyIndex :type Integer))
  (set `self.IsTilting` false))

(event `self.ReceiveTick`
  (params (DeltaSeconds :type "Float (single-precision)"))
  (bind _returnvalue (* DeltaSeconds 0.1))
  (bind _cube (`self.Cube`))
  (bind _tiltspeed (`self.TiltSpeed`))
  (bind _roll (.roll (`SceneComponent.RelativeRotation` _cube)))
  (if (`self.IsTilting`)
    (`SceneComponent.K2_SetRelativeRotation` _cube (`KismetMathLibrary.MakeRotator` (`KismetMathLibrary.FInterpTo` _roll (`self.TiltAngle`) _returnvalue _tiltspeed)) false false)
    (else
      (`SceneComponent.K2_SetRelativeRotation` _cube (`KismetMathLibrary.MakeRotator` (`KismetMathLibrary.FInterpTo` _roll 0.0 _returnvalue _tiltspeed)) false false))))

(fn `UserConstructionScript`)